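; Dialogue Blueprint that creates a W_GFDialogue widget shortly after BeginPlay and plays through DT_Dialogue lines on screen automatically.
; A self-calling debug event fetches the row at RowIndex, writes its Text to the widget and increments the index after a fixed delay.
; It also reapplies the image's own dynamic material as its brush on each line, and stops advancing once no row is found.
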(event Custom|debugsystem
  (Development|PrintString "Hello")
  (bind _outrownames (DataTable|GetDataTableRowNames "/Game/DataTables/Dialogue/DT_Dialogue.DT_Dialogue"))
  (bind _returnvalue (Utilities|GetDataTableRow "/Game/DataTables/Dialogue/DT_Dialogue.DT_Dialogue" (Utilities|Array|Get(acopy) _outrownames (Variables|Default|GetRowIndex)))
    (:then
      (Rendering|Components|TextRender|SetText (Variables|/Game/DataTables/Dialogue/W_GFDialogue.W_GFDialogue_C|GetTextBlock (stale EventBeginPlay _output_get)) (.text _returnvalue))
      (bind _returnvalue_2 (Appearance|GetDynamicMaterial (Variables|/Game/DataTables/Dialogue/W_GFDialogue.W_GFDialogue_C|GetImage_58 (stale EventBeginPlay _output_get)) :!class /Script/UMG.Image))
      (Class|Image|SetBrushfromMaterial (Variables|/Game/DataTables/Dialogue/W_GFDialogue.W_GFDialogue_C|GetImage_58 (stale EventBeginPlay _output_get)) _returnvalue_2)
      (Utilities|FlowControl|Delay 2.0)
      (Math|Integer|IncrementInt (Variables|Default|GetRowIndex)
        (:%20%20
          (CallFunction|Debugsystem))))))

(event EventBeginPlay
  (Utilities|FlowControl|Delay 0.2)
  (bind _returnvalue (UserInterface|CreateWidget "/Game/DataTables/Dialogue/W_GFDialogue.W_GFDialogue_C"))
  (bind _output_get (Variables|Default|SetW_Dialogue _returnvalue))
  (UserInterface|Viewport|AddtoViewport _output_get 0)
  (CallFunction|Debugsystem))

(fn ConstructionScript)