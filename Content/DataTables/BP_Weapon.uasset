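; BP_Weapon is a weapon Blueprint that displays its type, element and damage range through text components.
; BeginPlay fills the text from the WeaponType and ElementType enums and the min and max damage.
; RandomizeValues raises minimum damage by a random amount, derives a maximum above it, then refreshes the text and calls SetMesh.
; SetMesh picks the body mesh from an array indexed by WeaponType, while disconnected mesh and material nodes remain unused.
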(event Custom|updateText
  (Rendering|Components|TextRender|SetText (Variables|Default|GetWeapon) (Utilities|Text|ToText(String) (Utilities|String|EnumtoString (Variables|Default|GetWeaponType))))
  (Rendering|Components|TextRender|SetText (Variables|Default|GetElemental) (Utilities|Text|ToText(String) (Utilities|String|EnumtoString (Variables|Default|GetElementType))))
  (Rendering|Components|TextRender|SetText (Variables|Default|GetDamage) (Utilities|Text|ToText(String) (Utilities|String|Append (Utilities|String|ToString(Integer) (Variables|Default|GetMin%20Damage)) " - " (Utilities|String|ToString(Integer) (Variables|Default|GetMaxDamage))))))

(event Custom|SetMesh
  (Components|StaticMesh|SetStaticMesh (Variables|Default|GetWeaponBody) (Utilities|Array|Get(acopy) (Variables|Default|GetWeaponMeshes) (Math|Conversions|ToInteger(Byte) (Variables|Default|GetWeaponType)))))

(event Custom|RandomizeValues
  (bind _output_get (Variables|Default|SetMin%20Damage (+ (Variables|Default|GetMin%20Damage) (Math|Random|RandomInteger 2))))
  (Variables|Default|SetMaxDamage (+ _output_get (Math|Random|RandomIntegerinRange 1 4)))
  (CallFunction|UpdateText)
  (CallFunction|SetMesh))

(event EventBeginPlay
  (CallFunction|UpdateText))

(fn ConstructionScript)