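; BP_PatrolRoute is a patrol route actor that supplies world-space waypoints from a Spline.
; GetPatrolPointLocation advances PatrolIndex by Direction through IncrementPatrolPointIndex, then returns that spline point's location.
; Direction flips to -1 when the index equals the point count, one past the last point.
; The lower-bound check that would flip Direction back to 1 is disconnected, so the intended ping-pong never reverses at the start.
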(event Custom|Increment%20Patrol%20Point%20Index
  (Variables|Default|SetPatrolIndex (+ (Variables|Default|GetPatrolIndex) (Variables|Default|GetDirection)))
  (if (== (Variables|Default|GetPatrolIndex) (Spline|GetNumberOfSplinePoints (Variables|Default|GetSpline)))
    ;[1 1 1] flip the direction
    (Variables|Default|SetDirection -1)))

(event EventBeginPlay)

(event Collision|EventActorBeginOverlap
  (params (OtherActor :type Actor%20Object%20Reference)))

(event EventTick
  (params (DeltaSeconds :type Float%20%28single-precision%29)))

(fn ConstructionScript)

(fn GetPatrolPointLocation
  (CallFunction|IncrementPatrolPointIndex)
  (return (Spline|GetLocationatSplinePoint (Variables|Default|GetSpline) (Variables|Default|GetPatrolIndex) "World")))