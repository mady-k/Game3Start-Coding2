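; Stone door trigger that registers player one standing on it and asks the door to open.
; When a BP_ThirdPersonCharacter overlaps, it sets Player1On on the BP_StoneDoor_Child found by class lookup, then after a short delay calls OpenDoor with that character as view target.
; The sphere switches to the arrow material after that call; ending overlap clears the flag and restores the base material.
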(event Custom|SteppedMaterial
  (Rendering|Material|SetMaterial (Variables|Default|GetSphere) 0 "/Engine/VREditor/UI/ArrowMaterial.ArrowMaterial"))

(event Custom|SteppedOffMaterial
  (Rendering|Material|SetMaterial (Variables|Default|GetSphere) 0 "/Game/VRS_LowPolyNature/Materials/MI_Base.MI_Base"))

(event Collision|EventActorBeginOverlap
  (params (OtherActor :type Actor%20Object%20Reference))
  (Utilities|Casting|CastToBP_ThirdPersonCharacter OtherActor)
  (bind _returnvalue (Actor|GetActorOfClass "/Game/Blueprints/BP_StoneDoor_Child.BP_StoneDoor_Child_C"))
  (Variables|/Game/Blueprints/BP_StoneDoor_Child.BP_StoneDoor_Child_C|SetPlayer1On _returnvalue true)
  (Utilities|FlowControl|Delay 0.2)
  (Default|OpenDoor _returnvalue OtherActor) ; new view target is the player
  (CallFunction|SteppedMaterial))

(event EventTick
  (params (DeltaSeconds :type Float%20%28single-precision%29))
  (|CallParentFunction DeltaSeconds) ; This node is disabled and will not be called.\nDrag off pins to build functionality.
)

(event Collision|EventActorEndOverlap
  (params (OtherActor :type Actor%20Object%20Reference))
  (Utilities|Casting|CastToBP_ThirdPersonCharacter OtherActor)
  (bind _returnvalue (Actor|GetActorOfClass "/Game/Blueprints/BP_StoneDoor_Child.BP_StoneDoor_Child_C"))
  (Variables|/Game/Blueprints/BP_StoneDoor_Child.BP_StoneDoor_Child_C|SetPlayer1On _returnvalue false)
  (CallFunction|SteppedOffMaterial))

(fn ConstructionScript
  (|CallParentFunction))