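; Trigger actor that acts as the Player 2 switch for the BP_StoneDoor_Child stone door.
; When a BP_ThirdPersonCharacter begins overlapping, it finds the door by class, sets Player2On and calls OpenDoor, passing the overlapping character.
; When the character leaves, it clears Player2On on the door without calling any other door function.
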(event EventBeginPlay
  (|CallParentFunction) ; This node is disabled and will not be called.\nDrag off pins to build functionality.
)

(event Collision|EventActorBeginOverlap
  (params (OtherActor :type Actor%20Object%20Reference))
  (Utilities|Casting|CastToBP_ThirdPersonCharacter OtherActor)
  (bind _returnvalue (Actor|GetActorOfClass "/Game/Blueprints/BP_StoneDoor_Child.BP_StoneDoor_Child_C"))
  (Variables|/Game/Blueprints/BP_StoneDoor_Child.BP_StoneDoor_Child_C|SetPlayer2On _returnvalue true)
  (Default|OpenDoor _returnvalue OtherActor) ; new view target is the player
)

(event EventTick
  (params (DeltaSeconds :type Float%20%28single-precision%29))
  (|CallParentFunction DeltaSeconds) ; This node is disabled and will not be called.\nDrag off pins to build functionality.
)

(event Collision|EventActorEndOverlap
  (params (OtherActor :type Actor%20Object%20Reference))
  (Utilities|Casting|CastToBP_ThirdPersonCharacter OtherActor)
  (bind _returnvalue (Actor|GetActorOfClass "/Game/Blueprints/BP_StoneDoor_Child.BP_StoneDoor_Child_C"))
  (Variables|/Game/Blueprints/BP_StoneDoor_Child.BP_StoneDoor_Child_C|SetPlayer2On _returnvalue false))

(fn ConstructionScript
  (|CallParentFunction))