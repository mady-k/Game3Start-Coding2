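; GM_Coding2, apparently a Game Mode, manages per-level saves using the current level name as the slot.
; BeginPlay loads or creates an SG_LevelSave2, restoring collected coins and any non-zero player position; slots holding another save class are deleted.
; Checkpoint stores the player transform and FinishedLevel resets it, both writing to disk through SaveGame.
; A zero location serves as the "no checkpoint" marker.
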(event Custom|SaveGame
  (bind _returnvalue (Game|GetCurrentLevelName true))
  (bind _returnvalue_2 (SaveGame|SaveGametoSlot (Variables|Default|GetLevelSave) _returnvalue))
  (if _returnvalue_2
    (Development|PrintString "saved")
    (else
      (Development|PrintString "could not save"))))

(event EventBeginPlay
  ;[1 1 1] is there a level save file for this level's name? if not, create one, so that we can start editing it. if there is - load and store it to the "Level Save" variable, so we can start editing it.
  (bind _returnvalue (Game|GetCurrentLevelName true))
  (bind _returnvalue_2 (SaveGame|DoesSaveGameExist _returnvalue))
  (if _returnvalue_2
    (bind _returnvalue_3 (SaveGame|LoadGamefromSlot _returnvalue))
    (bind _assg_level_save_2 (Utilities|Casting|CastToSG_LevelSave2 _returnvalue_3)
      (:then
        (bind _output_get (Variables|Default|SetLevelSave _assg_level_save_2))
        (Default|LoadCollectedCoins _output_get)
        (if (not (Class|KismetMathLibrary|EqualExactlyVectorVector (.location (Variables|/Game/Blueprints/NewSaves/SG_LevelSave2.SG_LevelSave2_C|GetPlayerTransform (Variables|Default|GetLevelSave))) "0, 0, 0")) ; If the value of player transform is not 0,0,0, move them to that spot.
          (Transformation|SetWorldTransform (Variables|/Script/Engine.Character|GetCapsuleComponent (Game|GetPlayerCharacter 0)) (Variables|/Game/Blueprints/NewSaves/SG_LevelSave2.SG_LevelSave2_C|GetPlayerTransform (Variables|Default|GetLevelSave)) false false)))
      (:CastFailed
        (SaveGame|DeleteGameinSlot _returnvalue) ; delete the old saves from different save types
      ))
    (else
      (bind _returnvalue_4 (SaveGame|CreateSaveGameObject "/Game/Blueprints/NewSaves/SG_LevelSave2.SG_LevelSave2_C"))
      (Variables|Default|SetLevelSave _returnvalue_4))))

(fn ConstructionScript)

(fn Checkpoint
  (params (Player%20Transform :type Transform))
  (Variables|/Game/Blueprints/NewSaves/SG_LevelSave2.SG_LevelSave2_C|SetPlayerTransform (Variables|Default|GetLevelSave) Player%20Transform) ; set the Player Transform var\non the Level Save
  (CallFunction|SaveGame))

(fn FinishedLevel
  (Variables|/Game/Blueprints/NewSaves/SG_LevelSave2.SG_LevelSave2_C|SetPlayerTransform (Variables|Default|GetLevelSave) "") ; reset player start location to 0,0,0,
  (CallFunction|SaveGame))