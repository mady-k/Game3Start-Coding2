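; SG_LevelSave2 is a level save object, apparently a SaveGame, that restores collected coins and opened doors.
; LoadCollectedCoins loops over the CollectedCoins references and calls LoadCollectedState on each valid one.
; LoadDoorState does the same for OpenDoors, calling Quietdoor on each valid door.
; An unconnected second coin loop, which would call LoadCollectedCoins recursively, never runs.
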(fn LoadCollectedCoins
  (if (> (Utilities|Array|Length (Variables|Default|GetCollectedCoins)) 0) ; do we have any coins that\n are already collected
    (for _array_element (Variables|Default|GetCollectedCoins)
      (Utilities|IsValid _array_element
        (:Is%20Valid
          (Default|LoadCollectedState _array_element))))))

(fn LoadDoorState
  (if (> (Utilities|Array|Length (Variables|Default|GetOpenDoors)) 0)
    (for _array_element (Variables|Default|GetOpenDoors)
      (Utilities|IsValid _array_element
        (:Is%20Valid
          (Default|Quietdoor _array_element))))))