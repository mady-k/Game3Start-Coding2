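; Bullet drop test actor that repeatedly simulates a gravity-affected projectile path from its Arrow component.
; BeginPlay runs CoolCalc every 0.2 seconds, stepping line traces by SimFrequency and adding downward acceleration after each miss.
; A hit plays a ping and spawns a butterfly emitter without ending the loop; the player cast feeds nothing.
; Each pass resets Velocity to the Arrow's location; older calculator and debug nodes are disconnected.
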(event Custom|BulletDropCalculator)

(event Custom|CoolCalc
  (Variables|Default|SetEnd (+ (Variables|Default|GetStart) (/ (Variables|Default|GetVelocity) (Math|Vector|MakeVector (Variables|Default|GetSim%20Frequency) 1.0 1.0))))
  (Utilities|FlowControl|ForLoopwithBreak 1 (Math|Float|Truncate (Variables|Default|GetSim%20Frequency))
    (:LoopBody
      (bind _returnvalue (Class|KismetSystemLibrary|LineTraceSinglebyProfile (Variables|Default|GetStart) (Variables|Default|GetEnd) "BlockAll" false 0 "None" true))
      (if _returnvalue
        (Audio|PlaySoundatLocation "/Engine/EngineSounds/1kSineTonePing.1kSineTonePing" (Variables|Default|GetEnd) "0, 0, 0" 1.0 1.0 0.0 0 0 0 0)
        (Effects|SpawnEmitteratLocation "/Game/Realistic_Starter_VFX_Pack_Vol2/Particles/Environment/P_Butterfly.P_Butterfly" (Variables|Default|GetEnd))
        (Utilities|Casting|CastToBP_ThirdPersonCharacter (Game|GetPlayerCharacter 0))
        (else
          (Variables|Default|SetStart (Variables|Default|GetEnd))
          (Variables|Default|SetVelocity (+ (Variables|Default|GetVelocity) (Math|Vector|MakeVector 0.0 0.0 (/ -9.8e+02 (Math|Float|Square (Variables|Default|GetSim%20Frequency))))))
          (Variables|Default|SetEnd (+ (Variables|Default|GetStart) (/ (Variables|Default|GetVelocity) (Variables|Default|GetSim%20Frequency)))))))
    (:Completed
      (Variables|Default|SetStart (Transformation|GetWorldLocation (Variables|Default|GetArrow)))
      (Variables|Default|SetVelocity (Variables|Default|GetStart)))))

(event Custom|CustomEvent)

(event EventBeginPlay
  (Variables|Default|SetStart (Transformation|GetWorldLocation (Variables|Default|GetArrow)))
  (Utilities|FlowControl|Sequence :!label _label
    (:then_0
      (CallFunction|CoolCalc)
      (Utilities|FlowControl|Delay 0.2)
      (goto _label))))

(fn ConstructionScript)

(fn ReallyCoolCalculator)