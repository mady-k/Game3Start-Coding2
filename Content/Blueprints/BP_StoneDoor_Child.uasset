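; Child stone door for two players that opens only when it is closed and both player flags are on.
; OpenDoor stores each player's camera, records the door in the game mode's level save, then blends the player views to the door.
; A timeline lowers the door mesh with camera shake and force feedback.
; After a short delay, views blend back to the stored cameras at twice the speed.
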(event EventBeginPlay)

(event Collision|EventActorBeginOverlap
  (params (OtherActor :type Actor%20Object%20Reference)))

(event EventTick
  (params (DeltaSeconds :type Float%20%28single-precision%29)))

(event EventOpenDoor
  (params (NewViewTarget :type Actor%20Object%20Reference) (PlayerID :type Integer))
  (bind _returnvalue (Class|GameplayStatics|GetPlayerControllerfromID PlayerID))
  (bind _blend_time (Variables|Default|GetBlend%20Time))
  (bind _returnvalue_2 (/ _blend_time 2.0))
  (if (== PlayerID 0)
    (Variables|Default|SetPlayer1Cam NewViewTarget)
    (else
      (Variables|Default|SetPlayer2Cam NewViewTarget)))
  (if (Math|Boolean|ANDBoolean (Variables|Default|GetClosed) (Variables|Default|GetPlayer1On) (Variables|Default|GetPlayer2On))
    (bind _asgm_coding_2 (Utilities|Casting|CastToGM_Coding2 (Game|GetGameMode)))
    (Utilities|Array|AddUnique (Variables|/Game/Blueprints/NewSaves/SG_LevelSave2.SG_LevelSave2_C|GetOpenDoors (Variables|/Game/Blueprints/NewSaves/GM_Coding2.GM_Coding2_C|GetLevelSave _asgm_coding_2)) self)
    ;[1 1 1] from player to door
    (Game|Player|SetViewTargetwithBlend _returnvalue self (Variables|Default|GetBlend%20Time) "VTBlend_Cubic" 0.0 true)
    (Utilities|FlowControl|Delay (Variables|Default|GetBlend%20Time))
    (Game|Feedback|ClientPlayForceFeedback (Game|GetPlayerController 1) "/Game/Input/ForceFeedback/FFE_DoorShake.FFE_DoorShake" "None" false false false)
    (Game|Feedback|ClientStartCameraShake (Game|GetPlayerController 0) "/Game/Blueprints/CameraShake/CS_DoorOpen.CS_DoorOpen_C" 1.0 "CameraLocal" "0, 0, 0")
    (bind _newtrack_0 (Timeline|Timeline_1 Play)
      (:Update
        (Transformation|SetRelativeLocation (Variables|Default|GetDoor) (Math|Vector|Lerp(Vector) "-50.000000,175.000000,-10.000000" "-50.000000,175.000000,-261.000000" _newtrack_0) false false))
      (:Finished
        (Utilities|FlowControl|Delay 2.0) ; waiting 2 seconds while the door opens
        ;[1 1 1] from door to player
        (Game|Player|SetViewTargetwithBlend _returnvalue (Variables|Default|GetPlayer1Cam) _returnvalue_2 "VTBlend_Cubic" 0.0 false) ; shift camera back to player
        (Game|Player|SetViewTargetwithBlend (Game|GetPlayerController 1) (Variables|Default|GetPlayer2Cam) _returnvalue_2 "VTBlend_Cubic" 0.0 false) ; shift camera back to player
      ))
    (else
      (Development|PrintString "Hello"))))

(fn ConstructionScript
  (|CallParentFunction))